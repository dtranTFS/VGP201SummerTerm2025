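; BP_EnemyCube is an FPS enemy actor that takes damage and is destroyed when its health runs out.
; Its AnyDamage event passes the amount to TakeDamage, which applies it through ACHealthComponent.
; TakeDamage destroys the actor if the component reports it dead, and otherwise prints the remaining health.
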(event `self.ReceiveAnyDamage`
  (params (Damage :type "Float (single-precision)") (DamageType :type "DamageType Object Reference") (InstigatedBy :type "Controller Object Reference") (DamageCauser :type "Actor Object Reference"))
  (`self.TakeDamage` Damage))

(fn `TakeDamage`
  (params (`Damage Amt` :type "Float (double-precision)"))
  (bind _ac_healthcomponent (`self.AC_HealthComponent`))
  (`/Game/FPS/Blueprints/Components/AC_HealthComponent.Damage` _ac_healthcomponent `Damage Amt`)
  (if (`/Game/FPS/Blueprints/Components/AC_HealthComponent.IsDead` _ac_healthcomponent)
    (`self.K2_DestroyActor`)
    (else
      (`KismetSystemLibrary.PrintString` (`KismetStringLibrary.Conv_DoubleToString` (`/Game/FPS/Blueprints/Components/AC_HealthComponent.GetHealth` _ac_healthcomponent))))))

(fn `UserConstructionScript`
  (`parent.UserConstructionScript`))