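; Enemy AI controller that runs the BT_EnemyAI behavior tree and supplies it with sight information.
; When PawnSensing sees any pawn, it writes a can-see flag and that pawn as the player target to the Blackboard.
; A retriggerable delay of twice the sensing interval acts as a lost-sight timeout, clearing both values once sightings stop.
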(event `self.ReceiveBeginPlay`
  (`self.RunBehaviorTree` "/Game/FPS/Blueprints/Enemies/AI/BT_EnemyAI.BT_EnemyAI"))

(event `self.PawnSensing.OnSeePawn`
  (params (Pawn :type "Pawn Object Reference"))
  (`self.SetCanSeePlayer` Pawn true)
  (`KismetSystemLibrary.RetriggerableDelay` (* (`PawnSensingComponent.SensingInterval` (`self.PawnSensing`)) 2.0))
  (`self.SetCanSeePlayer` null))

(fn `SetCanSeePlayer`
  (params (PlayerTarget :type "Object Object Reference") (CenSeePlayer :type Boolean))
  (bind _blackboard (`self.Blackboard`))
  (`BlackboardComponent.SetValueAsBool` _blackboard (`self.BBCanSeePlayer`) CenSeePlayer)
  (`BlackboardComponent.SetValueAsObject` _blackboard (`self.BBPlayerTarget`) PlayerTarget))

(fn `UserConstructionScript`)