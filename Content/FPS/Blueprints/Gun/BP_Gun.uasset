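; BP_Gun is a gun Blueprint that exposes damage, fire rate and maximum bullet distance through getter functions.
; Its OnShoot event passes start and end positions to a Shooting function, which only prints a debug message and does no trace or damage.
; BeginPlay, overlap, Tick and the construction script are empty.
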(event `/Game/FPS/Blueprints/Player/BPI_Gun.OnShoot`
  (params (`Start Position` :type "Vector Structure") (`End Position` :type "Vector Structure"))
  (`self.Shooting` `Start Position` `End Position`))

(fn `GetDamage`
  (returns (Damage :type "Float (double-precision)"))
  (return (`self.Damage`)))

(fn `GetFireRate`
  (returns (FireRate :type "Float (double-precision)"))
  (return (`self.FireRate`)))

(fn `GetMaxBulletDistance`
  (returns (MaxBulletDistance :type "Float (double-precision)"))
  (return (`self.MaxBulletDistance`)))

(fn `Shooting`
  (params (`Start Position` :type "Vector Structure") (`End Position` :type "Vector Structure"))
  (`KismetSystemLibrary.PrintString` "BP_Gun Shooting Called"))

(fn `UserConstructionScript`)