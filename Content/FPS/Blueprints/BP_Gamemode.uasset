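; FPS game mode Blueprint that keeps the score and a countdown timer and shows both on an on-screen menu widget.
; BeginPlay creates WBP_GameMenu, switches input to game-only with a hidden cursor, and seeds the initial values.
; Tick runs UpdateTimer, whose one-second Delay throttles the countdown; no zero check exists.
; UpdateScore adds an amount, refreshes the widget and returns the new total.
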(event `self.ReceiveBeginPlay`
  (bind _menu_ref (`self.Menu Ref`))
  (`KismetSystemLibrary.PrintString` (`self.StartingString`) true true (struct :`G` 0.66 :`B` 1.0 :`A` 1.0) 5.0)
  (`self.SpawnGameMenu`)
  (`/Game/FPS/Blueprints/GUI/GameMenu/WBP_GameMenu.SetTimer` _menu_ref (`self.GameTimer`))
  (`/Game/FPS/Blueprints/GUI/GameMenu/WBP_GameMenu.SetScore` _menu_ref (`self.Score`)))

(event `self.ReceiveTick`
  (params (DeltaSeconds :type "Float (single-precision)"))
  (`self.UpdateTimer`))

(fn `SpawnGameMenu`
  (bind _returnvalue (`GameplayStatics.GetPlayerController` 0))
  (bind _returnvalue_2 (`|CreateWidget` "/Game/FPS/Blueprints/GUI/GameMenu/WBP_GameMenu.WBP_GameMenu_C"))
  (bind _output_get (set `self.Menu Ref` _returnvalue_2))
  ; Adds to Screen
  (`UserWidget.AddToViewport` _output_get 0)
  (`WidgetBlueprintLibrary.SetInputMode_GameOnly` _returnvalue)
  (set `PlayerController.bShowMouseCursor` false _returnvalue))

(fn `UpdateScore`
  (params (`Score Amt` :type Integer))
  (returns (`New Score` :type Integer))
  (bind _output_get (set `self.Score` (+ (`self.Score`) `Score Amt`)))
  (`/Game/FPS/Blueprints/GUI/GameMenu/WBP_GameMenu.SetScore` (`self.Menu Ref`) _output_get)
  (return _output_get))

(fn `UserConstructionScript`)